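; Performance test actor that measures average frame rate while a large grid of static mesh actors exists in the level.
; Keys 1–5 pick which static mesh component gets attached to each plain Actor spawned by the TemporarySpawn macro.
; The macro starts a delayed cleanup before spawning, exposing per-actor, all-spawned and all-destroyed exec outputs.
; Tick counts frames during the run, and cleanup prints elapsed time and average FPS.
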(event EventBeginPlay
  (Components|Activation|SetActive (Variables|Default|GetCamera) true false))

(event Collision|EventActorBeginOverlap
  (params (OtherActor :type Actor%20Object%20Reference)))

(event EventTick
  (params (DeltaSeconds :type Float%20%28single-precision%29))
  (if (Variables|Default|GetIsRunningTest)
    (Math|Integer|IncrementInt (Variables|Default|GetFrames))))

(event Input|KeyboardEvents|SpaceBar
  (params (Key :type Key%20Structure :default "None"))
  (:Pressed
    (if (Variables|Default|GetIsRunningTest)
      (Development|PrintString "Already Testing"))))

(event Input|KeyboardEvents|1
  (params (Key :type Key%20Structure :default "None"))
  (:Pressed
    (if (not (Variables|Default|GetIsRunningTest))
      (Variables|Default|SetTest%20index 0)
      (bind (_spawned_actor _spawned_actor_transform) (Utilities|TemporarySpawn 100 100 100 200 2e+01)
        (:Objects%20Spawned
          (Development|PrintString (Utilities|String|BuildString(Integer) "" "Test started with " (Utilities|Array|Length (Variables|Default|GetSpawnedActors)) " objects"))
          (Variables|Default|SetIsRunningTest true)
          (Variables|Default|SetFrames 0)
          (Variables|Default|SetTestStartTime (Math|DateTime|Now)))
        (:Actor%20Spawned%20%28Attach%20Components%20here%29
          (switch int (Variables|Default|GetTest%20index)
            (:0
              (AddComponent|AddStaticMeshComponent _spawned_actor false _spawned_actor_transform))
            (:1
              (AddComponent|AddStaticMeshComponent _spawned_actor false _spawned_actor_transform))
            (:2
              (AddComponent|AddStaticMeshComponent _spawned_actor false _spawned_actor_transform))
            (:3
              (AddComponent|AddStaticMeshComponent _spawned_actor false _spawned_actor_transform))
            (:4
              (AddComponent|AddStaticMeshComponent _spawned_actor false _spawned_actor_transform))))
        (:Objects%20Destroyed
          (Variables|Default|SetIsRunningTest false)
          (Development|PrintString "Test Done")
          (Development|PrintString (Class|KismetStringLibrary|BuildStringDouble "" (Utilities|String|BuildString(Integer) "" "Had " (Variables|Default|GetFrames) " frames in ") (Class|KismetMathLibrary|GetTotalMilliseconds (- (Math|DateTime|Now) (Variables|Default|GetTestStartTime))) " milliseconds") true true "(R=1.000000,G=0.000000,B=0.107766,A=1.000000)" 4.0)
          (Development|PrintString (Class|KismetStringLibrary|BuildStringDouble "" "Average of " (/ (Variables|Default|GetFrames) (Math|Timespan|GetTotalSeconds (- (Math|DateTime|Now) (Variables|Default|GetTestStartTime)))) " frames per second") true true "(R=1.000000,G=0.000000,B=0.107766,A=1.000000)" 4.0))))))

(event Input|KeyboardEvents|2
  (params (Key :type Key%20Structure :default "None"))
  (:Pressed
    (if (not (Variables|Default|GetIsRunningTest))
      (Variables|Default|SetTest%20index 1)
      (bind (_spawned_actor _spawned_actor_transform) (Utilities|TemporarySpawn 100 100 100 200 2e+01)
        (:Objects%20Spawned
          (Development|PrintString (Utilities|String|BuildString(Integer) "" "Test started with " (Utilities|Array|Length (Variables|Default|GetSpawnedActors)) " objects"))
          (Variables|Default|SetIsRunningTest true)
          (Variables|Default|SetFrames 0)
          (Variables|Default|SetTestStartTime (Math|DateTime|Now)))
        (:Actor%20Spawned%20%28Attach%20Components%20here%29
          (switch int (Variables|Default|GetTest%20index)
            (:0
              (AddComponent|AddStaticMeshComponent _spawned_actor false _spawned_actor_transform))
            (:1
              (AddComponent|AddStaticMeshComponent _spawned_actor false _spawned_actor_transform))
            (:2
              (AddComponent|AddStaticMeshComponent _spawned_actor false _spawned_actor_transform))
            (:3
              (AddComponent|AddStaticMeshComponent _spawned_actor false _spawned_actor_transform))
            (:4
              (AddComponent|AddStaticMeshComponent _spawned_actor false _spawned_actor_transform))))
        (:Objects%20Destroyed
          (Variables|Default|SetIsRunningTest false)
          (Development|PrintString "Test Done")
          (Development|PrintString (Class|KismetStringLibrary|BuildStringDouble "" (Utilities|String|BuildString(Integer) "" "Had " (Variables|Default|GetFrames) " frames in ") (Class|KismetMathLibrary|GetTotalMilliseconds (- (Math|DateTime|Now) (Variables|Default|GetTestStartTime))) " milliseconds") true true "(R=1.000000,G=0.000000,B=0.107766,A=1.000000)" 4.0)
          (Development|PrintString (Class|KismetStringLibrary|BuildStringDouble "" "Average of " (/ (Variables|Default|GetFrames) (Math|Timespan|GetTotalSeconds (- (Math|DateTime|Now) (Variables|Default|GetTestStartTime)))) " frames per second") true true "(R=1.000000,G=0.000000,B=0.107766,A=1.000000)" 4.0))))))

(event Input|KeyboardEvents|3
  (params (Key :type Key%20Structure :default "None"))
  (:Pressed
    (if (not (Variables|Default|GetIsRunningTest))
      (Variables|Default|SetTest%20index 2)
      (bind (_spawned_actor _spawned_actor_transform) (Utilities|TemporarySpawn 100 100 100 200 2e+01)
        (:Objects%20Spawned
          (Development|PrintString (Utilities|String|BuildString(Integer) "" "Test started with " (Utilities|Array|Length (Variables|Default|GetSpawnedActors)) " objects"))
          (Variables|Default|SetIsRunningTest true)
          (Variables|Default|SetFrames 0)
          (Variables|Default|SetTestStartTime (Math|DateTime|Now)))
        (:Actor%20Spawned%20%28Attach%20Components%20here%29
          (switch int (Variables|Default|GetTest%20index)
            (:0
              (AddComponent|AddStaticMeshComponent _spawned_actor false _spawned_actor_transform))
            (:1
              (AddComponent|AddStaticMeshComponent _spawned_actor false _spawned_actor_transform))
            (:2
              (AddComponent|AddStaticMeshComponent _spawned_actor false _spawned_actor_transform))
            (:3
              (AddComponent|AddStaticMeshComponent _spawned_actor false _spawned_actor_transform))
            (:4
              (AddComponent|AddStaticMeshComponent _spawned_actor false _spawned_actor_transform))))
        (:Objects%20Destroyed
          (Variables|Default|SetIsRunningTest false)
          (Development|PrintString "Test Done")
          (Development|PrintString (Class|KismetStringLibrary|BuildStringDouble "" (Utilities|String|BuildString(Integer) "" "Had " (Variables|Default|GetFrames) " frames in ") (Class|KismetMathLibrary|GetTotalMilliseconds (- (Math|DateTime|Now) (Variables|Default|GetTestStartTime))) " milliseconds") true true "(R=1.000000,G=0.000000,B=0.107766,A=1.000000)" 4.0)
          (Development|PrintString (Class|KismetStringLibrary|BuildStringDouble "" "Average of " (/ (Variables|Default|GetFrames) (Math|Timespan|GetTotalSeconds (- (Math|DateTime|Now) (Variables|Default|GetTestStartTime)))) " frames per second") true true "(R=1.000000,G=0.000000,B=0.107766,A=1.000000)" 4.0))))))

(event Input|KeyboardEvents|4
  (params (Key :type Key%20Structure :default "None"))
  (:Pressed
    (if (not (Variables|Default|GetIsRunningTest))
      (Variables|Default|SetTest%20index 3)
      (bind (_spawned_actor _spawned_actor_transform) (Utilities|TemporarySpawn 100 100 100 200 2e+01)
        (:Objects%20Spawned
          (Development|PrintString (Utilities|String|BuildString(Integer) "" "Test started with " (Utilities|Array|Length (Variables|Default|GetSpawnedActors)) " objects"))
          (Variables|Default|SetIsRunningTest true)
          (Variables|Default|SetFrames 0)
          (Variables|Default|SetTestStartTime (Math|DateTime|Now)))
        (:Actor%20Spawned%20%28Attach%20Components%20here%29
          (switch int (Variables|Default|GetTest%20index)
            (:0
              (AddComponent|AddStaticMeshComponent _spawned_actor false _spawned_actor_transform))
            (:1
              (AddComponent|AddStaticMeshComponent _spawned_actor false _spawned_actor_transform))
            (:2
              (AddComponent|AddStaticMeshComponent _spawned_actor false _spawned_actor_transform))
            (:3
              (AddComponent|AddStaticMeshComponent _spawned_actor false _spawned_actor_transform))
            (:4
              (AddComponent|AddStaticMeshComponent _spawned_actor false _spawned_actor_transform))))
        (:Objects%20Destroyed
          (Variables|Default|SetIsRunningTest false)
          (Development|PrintString "Test Done")
          (Development|PrintString (Class|KismetStringLibrary|BuildStringDouble "" (Utilities|String|BuildString(Integer) "" "Had " (Variables|Default|GetFrames) " frames in ") (Class|KismetMathLibrary|GetTotalMilliseconds (- (Math|DateTime|Now) (Variables|Default|GetTestStartTime))) " milliseconds") true true "(R=1.000000,G=0.000000,B=0.107766,A=1.000000)" 4.0)
          (Development|PrintString (Class|KismetStringLibrary|BuildStringDouble "" "Average of " (/ (Variables|Default|GetFrames) (Math|Timespan|GetTotalSeconds (- (Math|DateTime|Now) (Variables|Default|GetTestStartTime)))) " frames per second") true true "(R=1.000000,G=0.000000,B=0.107766,A=1.000000)" 4.0))))))

(event Input|KeyboardEvents|5
  (params (Key :type Key%20Structure :default "None"))
  (:Pressed
    (if (not (Variables|Default|GetIsRunningTest))
      (Variables|Default|SetTest%20index 4)
      (bind (_spawned_actor _spawned_actor_transform) (Utilities|TemporarySpawn 100 100 100 200 2e+01)
        (:Objects%20Spawned
          (Development|PrintString (Utilities|String|BuildString(Integer) "" "Test started with " (Utilities|Array|Length (Variables|Default|GetSpawnedActors)) " objects"))
          (Variables|Default|SetIsRunningTest true)
          (Variables|Default|SetFrames 0)
          (Variables|Default|SetTestStartTime (Math|DateTime|Now)))
        (:Actor%20Spawned%20%28Attach%20Components%20here%29
          (switch int (Variables|Default|GetTest%20index)
            (:0
              (AddComponent|AddStaticMeshComponent _spawned_actor false _spawned_actor_transform))
            (:1
              (AddComponent|AddStaticMeshComponent _spawned_actor false _spawned_actor_transform))
            (:2
              (AddComponent|AddStaticMeshComponent _spawned_actor false _spawned_actor_transform))
            (:3
              (AddComponent|AddStaticMeshComponent _spawned_actor false _spawned_actor_transform))
            (:4
              (AddComponent|AddStaticMeshComponent _spawned_actor false _spawned_actor_transform))))
        (:Objects%20Destroyed
          (Variables|Default|SetIsRunningTest false)
          (Development|PrintString "Test Done")
          (Development|PrintString (Class|KismetStringLibrary|BuildStringDouble "" (Utilities|String|BuildString(Integer) "" "Had " (Variables|Default|GetFrames) " frames in ") (Class|KismetMathLibrary|GetTotalMilliseconds (- (Math|DateTime|Now) (Variables|Default|GetTestStartTime))) " milliseconds") true true "(R=1.000000,G=0.000000,B=0.107766,A=1.000000)" 4.0)
          (Development|PrintString (Class|KismetStringLibrary|BuildStringDouble "" "Average of " (/ (Variables|Default|GetFrames) (Math|Timespan|GetTotalSeconds (- (Math|DateTime|Now) (Variables|Default|GetTestStartTime)))) " frames per second") true true "(R=1.000000,G=0.000000,B=0.107766,A=1.000000)" 4.0))))))

(fn ConstructionScript)